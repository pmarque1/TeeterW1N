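; Weeping Angel-style character that chases player 0 and freezes its movement and animation when its IsMoving flag is set.
; Tick resumes the chase whenever the flag is clear and resets it after each freeze, so nothing in this graph sets it true.
; It also carries player-style logic: camera angle and FPS/top-down toggles, clamped damage, and a resource count printout.
; The cursor and movement helper functions are empty stubs, and the tree spawn is unconnected.
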(event Game|Damage|EventAnyDamage
  (params (Damage :type Float%20%28single-precision%29) (DamageType :type Damage%20Type%20Object%20Reference) (InstigatedBy :type Controller%20Object%20Reference) (DamageCauser :type Actor%20Object%20Reference))
  (Variables|Default|Sethealth (Math|Float|Clamp(Float) (- (Variables|Default|Gethealth) Damage) 0.0 (Variables|Default|GetmaxHealth))))

(event EventTick
  (params (DeltaSeconds :type Float%20%28single-precision%29))
  (Development|PrintString (Utilities|String|ToString(Boolean) (Variables|Default|GetIsMoving)))
  (if (Variables|Default|GetIsMoving)
    (AI|Navigation|StopMovement (Pawn|GetController))
    (Variables|/Script/Engine.SkeletalMeshComponent|SetGlobalAnimRateScale (Variables|Character|GetMesh) 0.0)
    (Variables|/Script/Engine.CharacterMovementComponent|SetMaxWalkSpeed (Variables|Character|GetCharacterMovement) 0.0)
    (Variables|Default|SetIsMoving false)
    (else
      (AI|Navigation|SimpleMovetoLocation (Pawn|GetController) (Transformation|GetActorLocation (Game|GetPlayerCharacter 0)))
      (Variables|/Script/Engine.SkeletalMeshComponent|SetGlobalAnimRateScale (Variables|Character|GetMesh) 1.0)
      (Variables|/Script/Engine.CharacterMovementComponent|SetMaxWalkSpeed (Variables|Character|GetCharacterMovement) 1e+02))))

(event Input|KeyboardEvents|F
  (params (Key :type Key%20Structure :default "None"))
  (bind _springarm (Variables|Camera|GetSpringArm))
  (:Pressed
    (Utilities|FlowControl|FlipFlop
      (:A
        (Transformation|SetRelativeRotation _springarm "-90.000000, 0, 0" false false))
      (:B
        (Transformation|SetRelativeRotation _springarm "-50.000000, 0, 0" false false)))))

(event Input|KeyboardEvents|T
  (params (Key :type Key%20Structure :default "None"))
  (bind _returnvalue (Game|GetPlayerController 0))
  (:Pressed
    (Utilities|FlowControl|FlipFlop
      (:A
        (CameraFades|StartCameraFade :self (Game|GetPlayerCameraManager 0) :FromAlpha 1.0 :Duration 0.7)
        (Game|Player|SetViewTargetwithBlend (Game|GetPlayerController 0) self 1.0 "VTBlend_EaseIn" 0.0 false)
        (Components|Activation|SetActive (Variables|Default|GetFPS_Camera) true false)
        (Components|Activation|SetActive (Variables|Camera|GetCamera) false false)
        (Variables|Default|SetbUseControllerRotationYaw true)
        (Variables|Default|SetIsFPS true)
        (Variables|/Script/Engine.PlayerController|SetbShowMouseCursor _returnvalue false))
      (:B
        (Components|Activation|SetActive (Variables|Camera|GetCamera) true false)
        (Components|Activation|SetActive (Variables|Default|GetFPS_Camera) false false)
        (Variables|Default|SetbUseControllerRotationYaw false)
        (Variables|Default|SetIsFPS false)
        (Variables|/Script/Engine.PlayerController|SetbShowMouseCursor _returnvalue true)
        (Development|PrintText "Switch Trigger")))))

(event Input|KeyboardEvents|Q
  (params (Key :type Key%20Structure :default "None"))
  ;[1 1 1] Press "Q" to see how much you have collected
  (:Pressed
    (Development|PrintString (Utilities|String|Append "Wood Collected: " (Utilities|String|ToString(Integer) (Variables|Default|GetWoodAmount))))
    (Development|PrintString (Utilities|String|Append "Food Collected: " (Utilities|String|ToString(Integer) (Variables|Default|GetFoodAmount))))))

(fn ConstructionScript)

(fn MovetoHitLocation
  (params (Location :type Vector)))

(fn FollowMouseorFinger
  (params (Location :type Vector)))

(fn GetLocationUnderCursor
  (return "0, 0, 0"))

(fn GetLocationUnderFinger
  (return "0, 0, 0"))