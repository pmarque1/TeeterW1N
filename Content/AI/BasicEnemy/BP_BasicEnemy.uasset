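; Basic enemy that chases the player character and damages it at close range.
; Any PawnSensing sighting sets IsSeeingPlayer, which is never cleared here, and issues an AI MoveTo toward player 0.
; HurtBox overlaps with BP_TopDownCharacter toggle InRange.
; While in range, Tick subtracts directly from the player's Health, using a flag and Delay as the attack cooldown.
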(event OnSeePawn(PawnSensing)
  (params (Pawn :type Pawn%20Object%20Reference))
  (Variables|Default|SetisSeeingPlayer true)
  (CallFunction|FollowPlayer))

(event OnComponentBeginOverlap(HurtBox)
  (params (OverlappedComponent :type Primitive%20Component%20Object%20Reference) (OtherActor :type Actor%20Object%20Reference) (OtherComp :type Primitive%20Component%20Object%20Reference) (OtherBodyIndex :type Integer) (bFromSweep :type Boolean) (SweepResult :type Hit%20Result%20Structure%20%28by%20ref%29))
  (Utilities|Casting|CastToBP_TopDownCharacter OtherActor)
  (Variables|Default|SetinRange true))

(event OnComponentEndOverlap(HurtBox)
  (params (OverlappedComponent :type Primitive%20Component%20Object%20Reference) (OtherActor :type Actor%20Object%20Reference) (OtherComp :type Primitive%20Component%20Object%20Reference) (OtherBodyIndex :type Integer))
  (Utilities|Casting|CastToBP_TopDownCharacter OtherActor)
  (Variables|Default|SetinRange false))

(event Custom|FollowPlayer
  (if (Variables|Default|GetisSeeingPlayer)
    (AI|AIMoveTo self "0, 0, 0" (Game|GetPlayerCharacter 0) 5.0 false)))

(event EventTick
  (params (DeltaSeconds :type Float%20%28single-precision%29))
  (bind _asbp_top_down_character (Utilities|Casting|CastToBP_TopDownCharacter (Game|GetPlayerCharacter 0)))
  (if (not (Variables|Default|GethasAttackedRecently))
    (if (Variables|Default|GetinRange)
      (Variables|/Game/TopDown/Blueprints/BP_TopDownCharacter.BP_TopDownCharacter_C|Sethealth _asbp_top_down_character (- (Variables|/Game/TopDown/Blueprints/BP_TopDownCharacter.BP_TopDownCharacter_C|Gethealth _asbp_top_down_character) 1e+01))
      (Variables|Default|SethasAttackedRecently true)
      (Utilities|FlowControl|Delay 1.5)
      (Variables|Default|SethasAttackedRecently false))))

(fn ConstructionScript)